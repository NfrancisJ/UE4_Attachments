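; BP_PlayerCharacter is the player character for an attachment prototype that simulates VR hand attachment with a mouse.
; On BeginPlay it spawns a hand dummy and an attachment base, then each Tick moves the hand to a camera-to-cursor trace hit.
; Left click spawns a hand copy there, attached to the base with world transform kept.
; Input also drives held-button orbit, wheel zoom and E-held base rotation.
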(event `InputAction|ActivateMouse`
  (params (Key :type "Key Structure"))
  ;[0 0 0 1 24] Controls
  (:`Pressed`
    (set `self.bActivateOrbit` true))
  (:`Released`
    (set `self.bActivateOrbit` false)))

(event `InputAxis|MouseXOrbit`
  (params (AxisValue :type "Float (single-precision)"))
  ;[0 0 0 1 24] Controls
  (`self.AddControllerYawInput` (* (`KismetMathLibrary.Conv_BoolToInt` (`self.bActivateOrbit`)) AxisValue)))

(event `InputAxis|MouseYOrbit`
  (params (AxisValue :type "Float (single-precision)"))
  ;[0 0 0 1 24] Controls
  (`self.AddControllerPitchInput` (* (`KismetMathLibrary.Conv_BoolToInt` (`self.bActivateOrbit`)) AxisValue)))

(event `InputAxisKey|MouseWheelAxis`
  (params (AxisValue :type "Float (single-precision)"))
  (bind _springarm (`self.SpringArm`))
  ;[0 0 0 1 24] Controls
  (set `SpringArmComponent.TargetArmLength` (+ (`SpringArmComponent.TargetArmLength` _springarm) (* -30 AxisValue)) _springarm))

(event `Key|E`
  (params (Key :type "Key Structure"))
  (bind _rotatingmovement (`/Game/AttachmentRND/Blueprints/Interactable/BP_AttachmentBase.RotatingMovement` (`self.BaseObject`)))
  ;[0 0 0 1 24] Rotate Base Object
  (:`Pressed`
    (`ActorComponent.Activate` _rotatingmovement false))
  (:`Released`
    (`ActorComponent.Deactivate` _rotatingmovement)))

(event `Key|LeftMouseButton`
  (params (Key :type "Key Structure"))
  (:`Pressed`
    (bind _returnvalue (`|SpawnActorFromClass` "/Game/AttachmentRND/Blueprints/Core/BP_VRHandDummy.BP_VRHandDummy_C" (`self.HandDummyLocation`) "AdjustIfPossibleButAlwaysSpawn" "OverrideRootScale" null null))
    (`self.K2_AttachToActor` _returnvalue (`self.BaseObject`) "None" "KeepWorld" "KeepWorld" "KeepWorld" false)))

(event `self.ReceiveBeginPlay`
  ;[0 0 0 1 30] This is the Dummy Hand to simulate VR attachment
  (bind _returnvalue (`|SpawnActorFromClass` "/Game/AttachmentRND/Blueprints/Core/BP_VRHandDummy.BP_VRHandDummy_C" (`KismetMathLibrary.MakeTransform` (200.0 0.0 200.0)) "AlwaysSpawn" "OverrideRootScale" null null))
  (set `self.HandDummy` _returnvalue)
  (bind _returnvalue_2 (`|SpawnActorFromClass` "/Game/AttachmentRND/Blueprints/Interactable/BP_AttachmentBase.BP_AttachmentBase_C" (`KismetMathLibrary.MakeTransform` (0.0 0.0 50.0) (struct) (2.0 2.0 2.0)) "Undefined" "OverrideRootScale" null null))
  (set `self.BaseObject` _returnvalue_2))

(event `self.ReceiveTick`
  (params (DeltaSeconds :type "Float (single-precision)"))
  (bind (_worldlocation _worlddirection) (`PlayerController.DeprojectMousePositionToWorld` (cast `/Game/AttachmentRND/Blueprints/Core/BP_PlayerController` (`GameplayStatics.GetPlayerController` 0) :!pure true)))
  ;[0 0 0 1 30] This is the Dummy Hand to simulate VR attachment
  (bind _outhit (`KismetSystemLibrary.LineTraceSingle` (`SceneComponent.K2_GetComponentLocation` (`self.Camera`)) (+ _worldlocation (* _worlddirection 2000)) "TraceTypeQuery1" true (`|MakeArray` (`self.HandDummy`)) "None" false))
  (bind (_bblockinghit _binitialoverlap _time _distance _location) (`GameplayStatics.BreakHitResult` _outhit))
  (`self.K2_SetActorLocation` (`self.HandDummy`) _location false false)
  (set `self.HandDummyLocation` (`KismetMathLibrary.Conv_VectorToTransform` _location)))

(fn `UserConstructionScript`)